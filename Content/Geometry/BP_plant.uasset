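; BP_plant is a growable crop actor that advances through mesh stages over time until it can be harvested.
; On begin play it shows the first mesh, loads the duration from PlantsStructure and calls CallLanded.
; Tick counts the remaining time down, stepping the phase and mesh at set fractions of that duration.
; Reaching the final phase sets CanHarvest, which stops the countdown.
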(event EventBeginPlay
  (CallFunction|Init)
  (Default|CallLanded self))

(event Collision|EventActorBeginOverlap
  (params (OtherActor :type Actor%20Object%20Reference)))

(event EventTick
  (params (DeltaSeconds :type Float%20%28single-precision%29))
  (bind _plants_structure (Variables|Default|Getplants%20structure))
  (if (not (Variables|Default|Getcan%20Harvest))
    (bind _output_get (Variables|Default|Setremain%20time (- (Variables|Default|Getremain%20time) DeltaSeconds)))
    (if (<= _output_get (Utilities|Select :Index (Variables|Default|Getcurrent%20phase) :Option%200 (* (.duration _plants_structure) 0.75) :Option%201 (* (.duration _plants_structure) 0.5) :Option%202 (* (.duration _plants_structure) 0.0)))
      (bind _output_get_2 (Variables|Default|Setcurrent%20phase (+ (Variables|Default|Getcurrent%20phase) 1)))
      (CallFunction|UpdateMesh)
      (if (== _output_get_2 3)
        (Variables|Default|Setcan%20Harvest true)))))

(fn ConstructionScript)

(fn UpdateMesh
  (Components|StaticMesh|SetStaticMesh (Variables|Default|Getplant) (Utilities|Array|Get(acopy) (.phase (Variables|Default|Getplants%20structure)) (Variables|Default|Getcurrent%20phase))))

(fn Init
  (bind _plants_structure (Variables|Default|Getplants%20structure))
  (Components|StaticMesh|SetStaticMesh (Variables|Default|Getplant) (Utilities|Array|Get(acopy) (.phase _plants_structure)))
  (Variables|Default|Setremain%20time (.duration _plants_structure)))